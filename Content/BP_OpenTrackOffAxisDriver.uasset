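; Actor that drives an off-axis projection actor from OpenTrack head tracking.
; When its OpenTrackPoseReceiver gets a head pose, it remaps the position with a pre-offset, non-uniform and uniform scale, then a post-offset, and writes it to the OffAxisActor's EyeRelativePosition.
; Head rotation is not used, and a receiver data timeout only prints an orange warning.
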(event OnReceivedHeadPose(OpenTrackPoseReceiver)
  (params (HeadPose :type Open%20Track%20Head%20Pose%20Structure))
  (bind _position (Utilities|Struct|BreakOpenTrackHeadPose HeadPose))
  (bind _preoffset (Variables|Default|GetPreOffset))
  (bind _scalenonuniform (Variables|Default|GetScaleNonUniform))
  (bind _scaleuniform (Variables|Default|GetScaleUniform))
  (bind _postoffset (Variables|Default|GetPostOffset))
  (bind _returnvalue (+ _position _preoffset))
  (bind _returnvalue_2 (* _returnvalue _scalenonuniform))
  (bind _returnvalue_3 (* _returnvalue_2 _scaleuniform))
  (bind _returnvalue_4 (+ _returnvalue_3 _postoffset))
  (bind (_x _y _z) (Math|Vector|BreakVector _returnvalue_4))
  (Variables|/OffAxisProjection/OffAxisActor_Manual.OffAxisActor_Manual_C|SetEyeRelativePosition (Variables|Default|GetOffAxisActor) (Math|Vector|MakeVector _x _y _z)))

(event OnStartedListening(OpenTrackPoseReceiver)
  (params (ListenIp :type String) (ListenPort :type Integer)))

(event OnStoppedListening(OpenTrackPoseReceiver))

(event OnNoDataTimeout(OpenTrackPoseReceiver)
  (Development|PrintString "No data timeout reached!" true true "(R=1.000000,G=0.393028,B=0.000000,A=1.000000)"))

(event EventBeginPlay)

(event Collision|EventActorBeginOverlap
  (params (OtherActor :type Actor%20Object%20Reference)))

(event EventTick
  (params (DeltaSeconds :type Float%20%28single-precision%29)))

(fn ConstructionScript)